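; BP_PlayerActions is an input-enabled actor that lets the player hover over and edit tiles on the BP_Grid found at BeginPlay.
; Each tick it queries the grid for the tile under the cursor and, on a change, moves a tile state from the old tile to the new one if that exists.
; Pressing T tells the grid to swap the hovered tile's type.
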(event EventBeginPlay
  (bind _returnvalue (Actor|GetActorOfClass "/Game/Blueprints/Grid/BP_Grid.BP_Grid_C"))
  (Variables|Default|SetGrid _returnvalue)
  (Input|EnableInput (Game|GetPlayerController 0)))

(event EventTick
  (params (DeltaSeconds :type Float%20%28single-precision%29))
  (CallFunction|UpdateTileUnderCursor))

(event Input|MouseEvents|LeftMouseButton
  (params (Key :type Key%20Structure)))

(event Input|MouseEvents|RightMouseButton
  (params (Key :type Key%20Structure)))

(event Input|KeyboardEvents|T
  (params (Key :type Key%20Structure))
  (:Pressed
    (Default|SwapTileType (Variables|Default|GetGrid) (Variables|Default|GetHoverdTile))))

(fn ConstructionScript)

(fn UpdateTileUnderCursor
  (bind _index (Default|GetTileIndexUnderCursor (Variables|Default|GetGrid)))
  (if (!= _index (Variables|Default|GetHoverdTile))
    (Default|RemoveStatefromTile (Variables|Default|GetGrid) (Variables|Default|GetHoverdTile) "NewEnumerator1")
    (bind _output_get (Variables|Default|SetHoverdTile _index))
    (if (.ReturnValue (Utilities|Map|Find (Variables|/Game/Blueprints/Grid/BP_Grid.BP_Grid_C|GetGridTiles (Variables|Default|GetGrid)) _output_get))
      (Default|AddStatetoTile (Variables|Default|GetGrid) (Variables|Default|GetHoverdTile) "NewEnumerator1"))))