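; BP_GridVisual is the actor that renders a grid's tiles through a child BP_GridMeshInst instanced-mesh actor.
; Initialization stores the grid, sets up that child with a flat square mesh, border material and query-only collision, then places itself at the origin raised by a ground offset.
; Tile updates remove and re-add the instance by index with its transform, states and type, and destruction clears all instances.
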(event EventBeginPlay
  (Actor|Tick|SetActorTickEnabled false))

(fn ConstructionScript)

(fn InitializeGridVisual
  (params (Grid :type BP%20Grid%20Object%20Reference))
  (Variables|Default|SetGrid Grid)
  (Variables|Default|SetGridMeshInst (.AsBP%20Grid%20Mesh%20Inst (Utilities|Casting|CastToBP_GridMeshInst (Variables|/Script/Engine.ChildActorComponent|GetChildActor (Variables|Default|GetChildActor_GridMeshInst)))))
  (Default|InitializeGridMeshInst (Variables|Default|GetGridMeshInst) "/Game/Arts/SM_Grid_SquareFlat.SM_Grid_SquareFlat" "/Game/Arts/MI_Grid_Flat_Border.MI_Grid_Flat_Border" "(R=0.000000,G=0.000000,B=0.000000,A=1.000000)" "QueryOnly")
  (Transformation|SetActorLocation "0, 0, 0" false false)
  (CallFunction|SetOffsetfromGround (Variables|Default|GetOffsetFromGround)))

(fn SetOffsetfromGround
  (params (OffsetFromGround :type Float%20%28double-precision%29))
  (bind _returnvalue (Transformation|GetActorLocation))
  (Variables|Default|SetOffsetFromGround OffsetFromGround)
  (Transformation|SetActorLocation (Math|Vector|MakeVector (.x _returnvalue) (.y _returnvalue) (Variables|Default|GetOffsetFromGround)) false false))

(fn DestroyGridVisual
  (Utilities|IsValid (Variables|Default|GetGridMeshInst)
    (:Is%20Valid
      (Default|ClearInstance (Variables|Default|GetGridMeshInst)))))

(fn UpdateTileVisual
  (params (Data :type S%20Tile%20Data%20Structure))
  (Default|RemoveInstance (Variables|Default|GetGridMeshInst) (.index Data))
  (Default|AddInstance (Variables|Default|GetGridMeshInst) (.index Data) (.transform Data) (.states Data) (.tiletype Data)))