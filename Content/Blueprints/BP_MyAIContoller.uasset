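; BP_MyAIContoller is an AI controller that walks its controlled pawn along a supplied path, one tile at a time.
; MoveAlongPath stores the path, resets the index and calls MoveToNextTile.
; MoveToNextTile issues an AI MoveTo to the current point with a tight acceptance radius, then increments the index and calls itself again on success.
; The chain ends when the path is exhausted or a move fails, with no failure handling.
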(event Custom|MoveAlongPath
  (params (Path :type Array%20of%20Vectors))
  (Variables|Default|SetPathList Path)
  (Variables|Default|SetCurrentIndex 0)
  (CallFunction|MovetoNextTile))

(event Custom|MoveToNextTile
  (if (not (>= (Variables|Default|GetCurrentIndex) (Utilities|Array|Length (Variables|Default|GetPathList))))
    (AI|AIMoveTo (Pawn|GetControlledPawn) (Utilities|Array|Get(acopy) (Variables|Default|GetPathList) (Variables|Default|GetCurrentIndex)) 0 1e+01 false
      (:OnSuccess
        (Math|Integer|IncrementInt (Variables|Default|GetCurrentIndex)
          (:%20%20
            (CallFunction|MovetoNextTile)))))))

(fn ConstructionScript)