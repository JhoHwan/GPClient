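; BP_DebugMenu is a debug Blueprint that manages the on-screen WBP_DebugTap debug widget.
; ToggleDebugPanel flips a visibility flag, lazily creates the widget and adds it to the viewport if missing, then shows or hides it to match.
; BeginPlay calls the toggle once, so the widget is created at start with its visibility set by the flipped default.
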(event EventBeginPlay
  (CallFunction|ToggleDebugPanel))

(fn ConstructionScript)

(fn ToggleDebugPanel
  (Variables|Default|SetIsVisible (not (Variables|Default|GetIsVisible)))
  (Utilities|IsValid (Variables|Default|GetDebugMenu)
    (:Is%20Valid
      _)
    (:Is%20Not%20Valid
      (bind _returnvalue (UserInterface|CreateWidget "/Game/Blueprints/Debug/WBP_DebugTap.WBP_DebugTap_C"))
      (Variables|Default|SetDebugMenu _returnvalue)
      (UserInterface|Viewport|AddtoViewport (Variables|Default|GetDebugMenu) 0)))
  (Widget|SetVisibility (Variables|Default|GetDebugMenu) (select (Variables|Default|GetIsVisible) "Visible" "Hidden")))