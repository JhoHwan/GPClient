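; Player controller for click-to-move with a mouse-driven camera, using Enhanced Input and a visible cursor.
; A short click projects the cursor hit onto the navmesh, asks the possessed BP_Player to move there and spawns a cursor effect.
; Rotate input yaws the player's spring arm by mouse delta on Tick, while zoom input computes a target arm length.
; Follow and touch-location helpers are defined but never called here.
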(event Input|EnhancedActionEvents|EnhancedInputActionIA_SetDestination_Click
  (params (ActionValue :type Boolean) (ElapsedSeconds :type Float%20%28double-precision%29) (TriggeredSeconds :type Float%20%28double-precision%29) (InputAction :type Input%20Action%20Object%20Reference :default "/Game/Input/Actions/IA_SetDestination_Click.IA_SetDestination_Click"))
  (bind (_hit _location) (CallFunction|GetLocationUnderCursor))
  (:Canceled
    (if (< ElapsedSeconds (Variables|Input|GetPressedThreshold)) :!label _label
      (if _hit
        (CallFunction|Moveto _location))))
  (:Completed
    (goto _label)))

(event Input|EnhancedActionEvents|EnhancedInputActionIA_RotateCamera
  (params (ActionValue :type Boolean) (ElapsedSeconds :type Float%20%28double-precision%29) (TriggeredSeconds :type Float%20%28double-precision%29) (InputAction :type Input%20Action%20Object%20Reference :default "/Game/Input/Actions/IA_RotateCamera.IA_RotateCamera"))
  (:Triggered
    (Variables|Default|SetbIsRotatingCamera true))
  (:Completed
    (Variables|Default|SetbIsRotatingCamera false)))

(event Input|EnhancedActionEvents|EnhancedInputActionIA_ZoomCamera
  (params (ActionValue :type Float%20%28double-precision%29) (ElapsedSeconds :type Float%20%28double-precision%29) (TriggeredSeconds :type Float%20%28double-precision%29) (InputAction :type Input%20Action%20Object%20Reference :default "/Game/Input/Actions/IA_ZoomCamera.IA_ZoomCamera"))
  (:Triggered
    (Variables|Default|SetTargetArmLength (* ActionValue (+ (Variables|/Script/Engine.SpringArmComponent|GetTargetArmLength (Variables|/Game/Blueprints/BP_Player.BP_Player_C|GetSpringArm (Variables|Default|GetPlayeRef))) 1e+02)))))

(event EventPossess
  (params (PossessedPawn :type Pawn%20Object%20Reference))
  (bind _asbp_player (Utilities|Casting|CastToBP_Player (Game|Player|GetPlayerPawn 0)))
  (Variables|Default|SetPlayeRef _asbp_player))

(event EventBeginPlay
  (bind _returnvalue (PlayerController|LocalPlayerSubsystems|GetEnhancedInputLocalPlayerSubsystem))
  (Utilities|IsValid _returnvalue
    (:Is%20Valid
      (Input|AddMappingContext _returnvalue "/Game/Input/IMC_Default.IMC_Default" 0 "(bIgnoreAllPressedKeysUntilRelease=True,bForceImmediately=False,bNotifyUserSettings=False)")
      (Variables|Default|SetbShowMouseCursor true))))

(event EventTick
  (params (DeltaSeconds :type Float%20%28single-precision%29))
  (bind _playeref (Variables|Default|GetPlayeRef))
  (bind _springarm (Variables|/Game/Blueprints/BP_Player.BP_Player_C|GetSpringArm _playeref))
  (bind _returnvalue (Transformation|GetWorldRotation _springarm))
  (if (Variables|Default|GetbIsRotatingCamera)
    (Transformation|SetWorldRotation (Variables|/Game/Blueprints/BP_Player.BP_Player_C|GetSpringArm (Variables|Default|GetPlayeRef)) (Math|Rotator|MakeRotator (.roll _returnvalue) (.pitch _returnvalue) (+ (.yaw _returnvalue) (* (.DeltaX (Class|PlayerController|GetInputMouseDelta)) (Variables|Default|GetCameraRotatingSpeed)))) false false)))

(fn ConstructionScript)

(fn Moveto
  (params (Location :type Vector))
  (bind _playeref (Variables|Default|GetPlayeRef))
  (Utilities|IsValid _playeref
    (:Is%20Valid
      (Class|GPPlayer|RequestMove _playeref Location)
      (Niagara|SpawnSystematLocation (Variables|Input|GetFXCursor) Location))))

(fn Follow
  (params (Location :type Vector))
  (bind _returnvalue (Pawn|GetControlledPawn))
  (Pawn|Input|AddMovementInput _returnvalue (Math|Vector|GetUnitDirection(Vector) (Transformation|GetActorLocation _returnvalue) Location) 1.0 false))

(fn GetLocationUnderCursor
  (bind _returnvalue (Class|NavigationSystemV1|GetNavigationSystem))
  (bind _hitresult (Game|Player|GetHitResultUnderCursorbyChannel "TraceTypeQuery1" true))
  (bind _location (Collision|BreakHitResult _hitresult))
  (bind (_projectedlocation _returnvalue_2) (AI|Navigation|ProjectPointtoNavigation _returnvalue _location 0 0))
  (return _returnvalue_2 _projectedlocation))

(fn GetLocationUnderFinger
  (bind _hitresult (Class|PlayerController|GetHitResultUnderFingerbyChannel "Touch1" "TraceTypeQuery1" false))
  (bind (_bblockinghit _binitialoverlap _time _distance _location) (Collision|BreakHitResult _hitresult))
  (return _bblockinghit _location))